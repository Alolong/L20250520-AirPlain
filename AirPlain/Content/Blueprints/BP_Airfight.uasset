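; BP_Airfight is a player-flown aircraft pawn that steers by pitch and roll and fires rockets.
; On BeginPlay it registers its Right and Left components in the propeller component's list.
; Pitch and Roll axes apply clamped, delta-time-scaled local rotations, while FireRocket spawns BP_Rocket at the Arrow transform.
; A forward movement-input node is left unconnected, so this graph drives no forward motion.
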(event `self.ReceiveBeginPlay`
  (`KismetArrayLibrary.Array_Add` (`/Game/Blueprints/BP_PropellerConp.SceneComponent` (`self.BP_PropellerConp`)) (`self.Right`))
  (`KismetArrayLibrary.Array_Add` (`/Game/Blueprints/BP_PropellerConp.SceneComponent` (`self.BP_PropellerConp`)) (`self.Left`)))

(event `self.ReceiveTick`
  (params (DeltaSeconds :type "Float (single-precision)")))

(event `InputAction|FireRocket`
  (params (Key :type "Key Structure"))
  (:`Pressed`
    (`|SpawnActorFromClass` "/Game/Blueprints/BP_Rocket.BP_Rocket_C" (`SceneComponent.K2_GetComponentToWorld` (`self.Arrow`)) "Undefined" "MultiplyWithRoot" self (`Controller.K2_GetPawn` (`GameplayStatics.GetPlayerController` 0)))))

(event `InputAxis|Pitch`
  (params (AxisValue :type "Float (single-precision)"))
  (`self.K2_AddActorLocalRotation` (`KismetMathLibrary.MakeRotator` 0.0 (* (`KismetMathLibrary.FClamp` AxisValue -1.0) (`GameplayStatics.GetWorldDeltaSeconds`) 60.0))))

(event `InputAxis|Roll`
  (params (AxisValue :type "Float (single-precision)"))
  (`self.K2_AddActorLocalRotation` (`KismetMathLibrary.MakeRotator` (* (`KismetMathLibrary.FClamp` AxisValue -1.0) (`GameplayStatics.GetWorldDeltaSeconds`) 60.0))))

(fn `UserConstructionScript`)