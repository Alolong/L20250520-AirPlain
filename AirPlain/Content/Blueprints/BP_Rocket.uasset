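; BP_Rocket is a projectile that flies forward and explodes on overlap with another actor.
; Each tick it moves its Box component along local X by RocketSpeed scaled by delta time, rather than using a movement component.
; On overlap it spawns explosion particles and sound, calls ApplyDamage with its instigator's controller, then destroys itself.
; A short lifespan set at BeginPlay removes rockets that hit nothing.
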(event `self.ReceiveBeginPlay`
  (`self.SetLifeSpan` 4.0))

(event `self.ReceiveActorBeginOverlap`
  (params (OtherActor :type "Actor Object Reference"))
  (`GameplayStatics.SpawnEmitterAtLocation` "/Game/StarterContent/Particles/P_Explosion.P_Explosion" (`self.K2_GetActorLocation`))
  (`GameplayStatics.SpawnSoundAtLocation` "/Game/StarterContent/Audio/Explosion02.Explosion02" (`self.K2_GetActorLocation`) (struct) 1.0 1.0 0.0 null null)
  (`GameplayStatics.ApplyDamage` null 0.0 (`self.GetInstigatorController`) self)
  (`self.K2_DestroyActor`))

(event `self.ReceiveTick`
  (params (DeltaSeconds :type "Float (single-precision)"))
  (`SceneComponent.K2_AddLocalTransform` (`self.Box`) (`KismetMathLibrary.MakeTransform` (`KismetMathLibrary.MakeVector` (* (`GameplayStatics.GetWorldDeltaSeconds`) (`self.RocketSpeed`)))) false false))

(fn `UserConstructionScript`)